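; BP_StartTimer is a trigger volume that puts a timer widget on screen when the player walks into it.
; On the first overlap by player character 0, a DoOnce lets it create W_Timer, store it in WTimerRef and add it to the viewport.
; The construction script sizes BoxCollision from the BoxSize variable.
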(event OnComponentBeginOverlap(BoxCollision)
  (params (OverlappedComponent :type Primitive%20Component%20Object%20Reference) (OtherActor :type Actor%20Object%20Reference) (OtherComp :type Primitive%20Component%20Object%20Reference) (OtherBodyIndex :type Integer) (bFromSweep :type Boolean) (SweepResult :type Hit%20Result%20Structure%20%28by%20ref%29))
  (if (== OtherActor (Game|GetPlayerCharacter 0))
    (Utilities|FlowControl|DoOnce false
      (:Completed
        (bind _returnvalue (UserInterface|CreateWidget "/Game/Blueprints/w_Timer.w_Timer_C"))
        (bind _output_get (Variables|Public|SetW_TimerRef _returnvalue))
        (UserInterface|Viewport|AddtoViewport _output_get 0)))))

(fn ConstructionScript
  (Components|Box|SetBoxExtent (Variables|Default|GetBoxCollision) (Variables|Default|GetBox%20Size) true))