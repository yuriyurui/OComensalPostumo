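; Actor component that line traces from the player camera every Tick to find the BP_InteractArea being looked at.
; Trace acts on a hit only when the hit actor changes, using an exact class match that excludes child classes.
; TraceInteractArea toggles focus on and off as the target changes and caches the focused area.
; TryToInteract reads that area's InteractDuration, but the interaction itself is not implemented.
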(event Custom|TryToInteract
  (params (Input :type Boolean))
  (if Input
    (if (Variables|Default|GetisTracingIntArea)
      (bind _output_get (Variables|Default|SetInteract%20Duration (Variables|/Game/Blueprints/Interact/BP_InteractArea.BP_InteractArea_C|GetInteractDuration (Variables|Default|GetFocusedIntArea))))
      (if (> _output_get 0.0)
        _))))

(event EventBeginPlay)

(event EventTick
  (params (DeltaSeconds :type Float%20%28single-precision%29))
  (CallFunction|Trace))

(fn Trace
  (bind _returnvalue (Game|GetPlayerCameraManager 0))
  (bind _returnvalue_2 (Transformation|GetActorLocation _returnvalue))
  (bind (_outhit _returnvalue_3) (Collision|LineTraceByChannel _returnvalue_2 (+ _returnvalue_2 (* (Math|Vector|GetForwardVector (Transformation|GetActorRotation _returnvalue)) (Variables|Default|GetLenght))) "TraceTypeQuery1" false 0 "None"))
  (if _returnvalue_3
    (if (!= (Variables|Default|GetFocusedActor) (.HitActor (Collision|BreakHitResult _outhit)))
      (Variables|Default|SetFocusedActor (.HitActor (Collision|BreakHitResult _outhit)))
      (CallFunction|TraceInteractArea (== (Utilities|GetClass (.HitActor (Collision|BreakHitResult _outhit))) "/Game/Blueprints/Interact/BP_InteractArea.BP_InteractArea_C")))
    (else
      (CallFunction|TraceInteractArea false))))

(fn TraceInteractArea
  (params (Trace :type Boolean))
  (if Trace
    (if (Variables|Default|GetisTracingIntArea)
      (Default|ToggleFocus (Variables|Default|GetFocusedIntArea) false))
    (bind _asbp_interact_area (Utilities|Casting|CastToBP_InteractArea (Variables|Default|GetFocusedActor)))
    (bind _output_get (Variables|Default|SetFocusedIntArea _asbp_interact_area))
    (Default|ToggleFocus _output_get true)
    (Variables|Default|SetisTracingIntArea true)
    (elif (Variables|Default|GetisTracingIntArea)
      (Variables|Default|SetisTracingIntArea false)
      (Default|ToggleFocus (Variables|Default|GetFocusedIntArea) false)
      (Variables|Default|SetFocusedActor 0)
      (Variables|Default|SetFocusedIntArea 0))))