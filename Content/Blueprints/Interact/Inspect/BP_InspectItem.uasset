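; Inspection actor that shows an item's mesh through a scene capture for the player to examine.
; Inspect sets the mesh, adds the name/description widget and moves input from the character to itself.
; Left-drag rotates, the wheel zooms via capture FOV, and right-click resets both; WASD rotation is multiplied by zero.
; Interact re-enables player input, removes the widget and destroys the actor.
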(event Custom|SetInspectRotation
  (params (ItemRotation :type Rotator))
  (bind _item (Variables|Default|GetItem))
  (bind _returnvalue (Transformation|GetWorldTransform _item))
  ;[0.15 0.15 0.15 0.5] Set Inspect Rotation (dinamically)
  (Variables|Default|SetInitial%20Item%20Rotation ItemRotation)
  (Transformation|SetWorldTransform _item (Math|Transform|MakeTransform (.location _returnvalue) (.rotation _returnvalue) (.scale _returnvalue)) false false))

(event Custom|SetInspectScale
  (params (InspectScale :type Vector))
  (bind _item (Variables|Default|GetItem))
  (bind _returnvalue (Transformation|GetWorldTransform _item))
  ;[0.15 0.15 0.15 0.5] Set Inspect Scale (dinamically)
  (Transformation|SetWorldTransform _item (Math|Transform|MakeTransform (.location _returnvalue) (.rotation _returnvalue) InspectScale) false false))

(event Input|EnhancedActionEvents|EnhancedInputActionIA_Interact
  (params (ActionValue :type Boolean) (ElapsedSeconds :type Float%20%28double-precision%29) (TriggeredSeconds :type Float%20%28double-precision%29) (InputAction :type Input%20Action%20Object%20Reference :default "/Game/Blueprints/Input/IA_Interact.IA_Interact"))
  (bind _returnvalue (Game|GetPlayerController 0))
  (:Started
    (Input|DisableInput (Variables|Default|GetCharacter) _returnvalue)
    (Input|EnableInput (Game|GetPlayerCharacter 0) _returnvalue)
    (Utilities|IsValid (Variables|Default|GetInspectWidgetRef)
      (:Is%20Valid
        (Widget|RemovefromParent (Variables|Default|GetInspectWidgetRef))
        (Variables|Default|SetInspectWidgetRef 0)
        (Actor|DestroyActor)))))

(event Input|EnhancedActionEvents|EnhancedInputActionIA_Move
  (params (ActionValue :type Vector%202D%20Structure) (ElapsedSeconds :type Float%20%28double-precision%29) (TriggeredSeconds :type Float%20%28double-precision%29) (InputAction :type Input%20Action%20Object%20Reference :default "/Game/Blueprints/Input/IA_Move.IA_Move"))
  ;[0.15 0.15 0.15 0.5] Move Item w/ WASD
  (if (or (!= (.x ActionValue) 0.0) (!= (.y ActionValue) 0.0))
    (Utilities|FlowControl|Sequence
      (:then_0
        (Transformation|SetWorldRotation (Variables|Default|GetItem) (Math|Rotator|CombineRotators (Transformation|GetWorldRotation (Variables|Default|GetItem)) (Math|Rotator|MakeRotator 0.0 0.0 (* (.x ActionValue) 0.0))) false false))
      (:then_1
        (Transformation|SetWorldRotation (Variables|Default|GetItem) (Math|Rotator|CombineRotators (Transformation|GetWorldRotation (Variables|Default|GetItem)) (Math|Rotator|MakeRotator 0.0 (* (.y ActionValue) 0.0) 0.0)) false false)))))

(event EventInspect
  (params (Character :type BP%20Player%20Object%20Reference) (InspectedItem :type Static%20Mesh%20Object%20Reference) (ItemName :type Text) (ItemDecript :type Text))
  (bind _returnvalue (Game|GetPlayerController 0))
  (Variables|Default|SetCharacter Character)
  (Components|StaticMesh|SetStaticMesh (Variables|Default|GetItem) InspectedItem)
  (bind _returnvalue_2 (UserInterface|CreateWidget "/Game/Blueprints/Interact/Inspect/UI_Inspect.UI_Inspect_C" 0 ItemName ItemDecript))
  (bind _output_get (Variables|Default|SetInspectWidgetRef _returnvalue_2))
  (UserInterface|Viewport|AddtoViewport _output_get 0)
  (Input|DisableInput (Variables|Default|GetCharacter) _returnvalue)
  (Input|EnableInput _returnvalue))

(event Input|MouseEvents|MouseX
  (params (AxisValue :type Float%20%28single-precision%29))
  ;[0.15 0.15 0.15 0.5] Set Inspect Horizontal Rotation
  (if (Variables|Default|GetRotate?)
    (Transformation|SetWorldRotation (Variables|Default|GetItem) (Math|Rotator|CombineRotators (Transformation|GetWorldRotation (Variables|Default|GetItem)) (Math|Rotator|MakeRotator 0.0 0.0 (* AxisValue -3.0))) false false)))

(event Input|MouseEvents|MouseY
  (params (AxisValue :type Float%20%28single-precision%29))
  ;[0.15 0.15 0.15 0.5] Set Inspect Vertical Rotation
  (if (Variables|Default|GetRotate?)
    (Transformation|SetWorldRotation (Variables|Default|GetItem) (Math|Rotator|CombineRotators (Transformation|GetWorldRotation (Variables|Default|GetItem)) (Math|Rotator|MakeRotator 0.0 (* AxisValue -3.0) 0.0)) false false)))

(event Input|MouseEvents|LeftMouseButton
  (params (Key :type Key%20Structure :default "None"))
  ;[0.15 0.15 0.15 0.5] Allow Inspection
  (:Pressed
    (Variables|Default|SetRotate? true))
  (:Released
    (Variables|Default|SetRotate? false)))

(event Input|MouseEvents|RightMouseButton
  (params (Key :type Key%20Structure :default "None"))
  ;[0.15 0.15 0.15 0.5] Reset Inspect Transform Rotation
  (:Pressed
    (Transformation|SetWorldRotation (Variables|Default|GetItem) (Variables|Default|GetInitial%20Item%20Rotation) false false)
    (Variables|/Script/Engine.SceneCaptureComponent2D|SetFOVAngle (Variables|Default|GetSceneCaptureComponent2D) 5e+01)))

(event Input|MouseEvents|MouseWheelUp
  (params (Key :type Key%20Structure :default "None"))
  (bind _scenecapturecomponent2d (Variables|Default|GetSceneCaptureComponent2D))
  ;[0.15 0.15 0.15 0.5] Zoom In
  (:Pressed
    (Variables|/Script/Engine.SceneCaptureComponent2D|SetFOVAngle _scenecapturecomponent2d (Math|Float|Clamp(Float) (- (Variables|/Script/Engine.SceneCaptureComponent2D|GetFOVAngle _scenecapturecomponent2d) 1.0) 3e+01 8e+01))))

(event Input|MouseEvents|MouseWheelDown
  (params (Key :type Key%20Structure :default "None"))
  (bind _scenecapturecomponent2d (Variables|Default|GetSceneCaptureComponent2D))
  ;[0.15 0.15 0.15 0.5] Zoom Out
  (:Pressed
    (Variables|/Script/Engine.SceneCaptureComponent2D|SetFOVAngle _scenecapturecomponent2d (Math|Float|Clamp(Float) (+ (Variables|/Script/Engine.SceneCaptureComponent2D|GetFOVAngle _scenecapturecomponent2d) 1.0) 3e+01 8e+01))))

(fn ConstructionScript)

(fn OnInteract
  (params (Character :type BP%20Player%20Object%20Reference))
  (return))