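; Base interactable item that can be inspected and collected toward an objective counter, with mesh, scale, icon position and detection radii set in the construction script.
; Inner and outer collision spheres toggle proximity billboards, though only the outer one checks for the player.
; While Inspect is set, interacting spawns a far-off BP_InspectItem and clears the flag.
; Otherwise it increments the objective widget, destroys itself, and pauses with a win menu at the limit.
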(event OnComponentBeginOverlap(innerCollision)
  (params (OverlappedComponent :type Primitive%20Component%20Object%20Reference) (OtherActor :type Actor%20Object%20Reference) (OtherComp :type Primitive%20Component%20Object%20Reference) (OtherBodyIndex :type Integer) (bFromSweep :type Boolean) (SweepResult :type Hit%20Result%20Structure%20%28by%20ref%29))
  ;[0.15 0.15 0.15 0.5] Player Detection (if they're in or out of the range)
  (if true
    (Rendering|SetVisibility (Variables|Default|GetouterBillboard) false false)
    (Rendering|SetVisibility (Variables|Default|GetinnerBillboard) true false)))

(event OnComponentEndOverlap(innerCollision)
  (params (OverlappedComponent :type Primitive%20Component%20Object%20Reference) (OtherActor :type Actor%20Object%20Reference) (OtherComp :type Primitive%20Component%20Object%20Reference) (OtherBodyIndex :type Integer))
  ;[0.15 0.15 0.15 0.5] Player Detection (if they're in or out of the range)
  (if true
    (Rendering|SetVisibility (Variables|Default|GetinnerBillboard) false false)
    (Rendering|SetVisibility (Variables|Default|GetouterBillboard) true false)))

(event OnComponentBeginOverlap(outerCollision)
  (params (OverlappedComponent :type Primitive%20Component%20Object%20Reference) (OtherActor :type Actor%20Object%20Reference) (OtherComp :type Primitive%20Component%20Object%20Reference) (OtherBodyIndex :type Integer) (bFromSweep :type Boolean) (SweepResult :type Hit%20Result%20Structure%20%28by%20ref%29))
  ;[0.15 0.15 0.15 0.5] Player Detection (if they're in or out of the range)
  (if (== OtherActor (Game|GetPlayerCharacter 0))
    (Rendering|SetVisibility (Variables|Default|GetouterBillboard) true false)))

(event OnComponentEndOverlap(outerCollision)
  (params (OverlappedComponent :type Primitive%20Component%20Object%20Reference) (OtherActor :type Actor%20Object%20Reference) (OtherComp :type Primitive%20Component%20Object%20Reference) (OtherBodyIndex :type Integer))
  ;[0.15 0.15 0.15 0.5] Player Detection (if they're in or out of the range)
  (if (== OtherActor (Game|GetPlayerCharacter 0))
    (Rendering|SetVisibility (Variables|Default|GetouterBillboard) false false)))

(event EventBeginPlay
  (bind _asbp_player (Utilities|Casting|CastToBP_Player (Game|GetPlayerCharacter 0)))
  (Variables|Public|Ref|SetplayerRef _asbp_player)
  (bind _returnvalue (Actor|GetActorOfClass "/Game/Blueprints/BP_ObjectivePoint.BP_ObjectivePoint_C"))
  (bind _asbp_objective_point (Utilities|Casting|CastToBP_ObjectivePoint _returnvalue))
  (bind _output_get (Variables|Default|SetBP_Objetivo _asbp_objective_point))
  (Variables|Default|SetW_Objetivo%20Ref (Variables|/Game/Blueprints/BP_ObjectivePoint.BP_ObjectivePoint_C|GetW_ObjectiveWidgetRef _output_get)))

(event EventOnInteract
  (params (Character :type BP%20Player%20Object%20Reference))
  (bind _w_objetivo_ref (Variables|Default|GetW_Objetivo%20Ref))
  (if (Variables|Public|Interaction|Inspection|GetInspect?)
    (bind _returnvalue (Game|SpawnActorfromClass "/Game/Blueprints/Interact/Inspect/BP_InspectItem.BP_InspectItem_C" (Math|Transform|MakeTransform "100000000.000000,0.000000,0.000000") "Undefined" "MultiplyWithRoot" 0 0))
    (Default|SetInspectRotation _returnvalue (Variables|Public|Interaction|Inspection|GetItemInspectRotation))
    (Default|SetInspectScale _returnvalue (Variables|Public|Interaction|Inspection|GetItemInspectScale))
    (Class|BIInteraction|Inspect(Message) _returnvalue Character (Variables|Public|Mesh|GetItemMesh) (Variables|Public|Mesh|GetItemName) (Variables|Public|Mesh|GetItemDescript))
    (Variables|Public|Interaction|Inspection|SetInspect? false)
    (else
      (Default|AddCounter _w_objetivo_ref)
      (if (Variables|/Game/Blueprints/W_Objetivo.W_Objetivo_C|GetatingiuLimite? _w_objetivo_ref)
        (Game|SetGamePaused true)
        (Variables|/Script/Engine.PlayerController|SetbShowMouseCursor (Game|GetPlayerController 0) true)
        (bind _returnvalue_2 (UserInterface|CreateWidget "/Game/Blueprints/W_MenuGanhou.W_MenuGanhou_C"))
        (UserInterface|Viewport|AddtoViewport _returnvalue_2 0)
        (Actor|DestroyActor)
        (else
          (Actor|DestroyActor))))))

(fn ConstructionScript
  (bind _staticmesh (Variables|Default|GetStaticMesh))
  (Utilities|FlowControl|Sequence
    (:then_0
      ;[0.15 0.15 0.15 0.5] Set Sphere Radius for Collision
      (Components|Sphere|SetSphereRadius (Variables|Default|GetinnerCollision) (Variables|Public|Interaction|Settings|GetInner%20Sphere%20Radius) true)
      (Components|Sphere|SetSphereRadius (Variables|Default|GetouterCollision) (Variables|Public|Interaction|Settings|GetOuter%20Sphere%20Radius) true)
      ;[0.15 0.15 0.15 0.5] Set Interaction Icon Location
      (Transformation|SetRelativeLocation (Variables|Default|GetinnerBillboard) (Variables|Public|Interaction|Settings|GetIconLocation) false false))
    (:then_1
      ;[0.15 0.15 0.15 0.5] Set Mesh (dinamically)
      (Components|StaticMesh|SetStaticMesh (Variables|Default|GetStaticMesh) (Variables|Public|Mesh|GetItemMesh))
      ;[0.15 0.15 0.15 0.5] Setting Mesh Scale (dinamically)
      (Transformation|SetWorldTransform _staticmesh (Math|Transform|MakeTransform (Transformation|GetWorldLocation _staticmesh) (Transformation|GetWorldRotation _staticmesh) (Variables|Public|Mesh|GetItemScale)) false false))
    (:then_2
      (if (Variables|Public|Interaction|Settings|GetDebugging?)
        (Rendering|SetVisibility (Variables|Default|GetinnerCollision) true false)
        (Rendering|SetVisibility (Variables|Default|GetouterCollision) true false)
        (else
          (Rendering|SetVisibility (Variables|Default|GetinnerCollision) false false)
          (Rendering|SetVisibility (Variables|Default|GetouterCollision) false false))))))

(fn Interact
  (params (Interactor :type Character%20Object%20Reference))
  (return false))