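; BP_Porta is an interactable door that swings open or closed and switches its nav modifier between default and null areas.
; OnInteract checks the player's hit actor; the first valid call only latches the swing side from a facing dot product.
; Later calls toggle the state, each applying a single FInterpTo yaw step, with no Tick or timeline in the graph.
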(event Custom|Handle%20Door%20Rotation
  (params (SetDoorRotation :type Float%20%28double-precision%29))
  (bind _door (Variables|Default|GetDoor))
  ;[0.15 0.15 0.15 0.5] Door Rotation Handler
  (Transformation|SetRelativeRotation _door (Math|Rotator|MakeRotator 0.0 0.0 (Math|Interpolation|FInterpTo (.Yaw (Math|Rotator|BreakRotator (Variables|/Script/Engine.SceneComponent|GetRelativeRotation _door))) SetDoorRotation (Utilities|Time|GetWorldDeltaSeconds) (Variables|Default|GetInterp%20Speed))) false false))

(event Custom|HandleDoor
  (bind _navmodifier (Variables|Default|GetNavModifier))
  ;[0.15 0.15 0.15 0.5] Handle Door
  (if (Variables|Default|GetisDoorOpened?)
    (CallFunction|HandleDoorRotation 0.0)
    (Variables|Default|SetisDoorOpened? false)
    (Class|NavModifierComponent|SetAreaClass _navmodifier "/Script/NavigationSystem.NavArea_Null")
    (else
      (CallFunction|HandleDoorRotation (* (Variables|Default|GetOpenDoorAngle) (Variables|Default|GetOpen%20Door%20Side)))
      (Variables|Default|SetisDoorOpened? true)
      (Class|NavModifierComponent|SetAreaClass _navmodifier "/Script/NavigationSystem.NavArea_Default"))))

(event Custom|Is%20Interacting%20With%20Door
  (params (Player :type BP%20Player%20Object%20Reference))
  (if (> (Math|Vector|DotProduct (Transformation|GetActorForwardVector Player) (Math|Vector|GetForwardVector (Variables|Default|GetOpenDoorLocation))) 0.0)
    (Variables|Default|SetOpen%20Door%20Side -1.0)
    (else
      (Variables|Default|SetOpen%20Door%20Side 1.0)))
  (Variables|Default|SetIsInteractingWDoor true))

(event EventBeginPlay
  (bind _asbp_player (Utilities|Casting|CastToBP_Player (Game|GetPlayerCharacter 0)))
  (Variables|Default|SetPlayer%20Ref _asbp_player))

(event EventOnInteract
  (params (Character :type BP%20Player%20Object%20Reference))
  (bind _player_ref (Variables|Default|GetPlayer%20Ref))
  (if (and (Variables|/Game/Blueprints/BP_Player.BP_Player_C|GetisInteracting _player_ref) (== (Variables|/Game/Blueprints/BP_Player.BP_Player_C|GetHit%20Actor _player_ref) self))
    (if (Variables|Default|GetIsInteractingWDoor)
      (CallFunction|HandleDoor)
      (else
        (CallFunction|IsInteractingwithDoor (Variables|Default|GetPlayer%20Ref))))))

(fn ConstructionScript)