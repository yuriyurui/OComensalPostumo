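; BP_Armario is a wardrobe hiding spot that tracks whether the player is hidden inside its box trigger.
; On BeginPlay it caches the BP_Porta door returned by GetActorOfClass.
; When the player enters the box, IsPlayerHidden is set from that door's IsDoorOpened state at that moment, and leaving clears it.
; The construction script sizes the trigger from ColliderSize.
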(event OnComponentBeginOverlap(Box)
  (params (OverlappedComponent :type Primitive%20Component%20Object%20Reference) (OtherActor :type Actor%20Object%20Reference) (OtherComp :type Primitive%20Component%20Object%20Reference) (OtherBodyIndex :type Integer) (bFromSweep :type Boolean) (SweepResult :type Hit%20Result%20Structure%20%28by%20ref%29))
  (if (== OtherActor (Game|GetPlayerCharacter 0))
    (if (Variables|/Game/Blueprints/BP_Porta.BP_Porta_C|GetisDoorOpened? (Variables|Default|GetPorta%20Ref))
      (Variables|Default|SetisPlayerHidden true)
      (else
        (Variables|Default|SetisPlayerHidden false)))))

(event OnComponentEndOverlap(Box)
  (params (OverlappedComponent :type Primitive%20Component%20Object%20Reference) (OtherActor :type Actor%20Object%20Reference) (OtherComp :type Primitive%20Component%20Object%20Reference) (OtherBodyIndex :type Integer))
  (if (== OtherActor (Game|GetPlayerCharacter 0))
    (Variables|Default|SetisPlayerHidden false)))

(event EventBeginPlay
  (bind _returnvalue (Actor|GetActorOfClass "/Game/Blueprints/BP_Porta.BP_Porta_C"))
  (bind _asbp_porta (Utilities|Casting|CastToBP_Porta _returnvalue))
  (Variables|Default|SetPorta%20Ref _asbp_porta))

(fn ConstructionScript
  (Components|Box|SetBoxExtent (Variables|Default|GetBox) (Variables|Default|GetColliderSize) true))