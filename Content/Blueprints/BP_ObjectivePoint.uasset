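; BP_ObjectivePoint is a trigger volume that shows an on-screen objective once the player leaves its box.
; It creates a W_Objetivo widget on BeginPlay, then a one-shot end-overlap sets its text and color, displays it with a fade and flags the objective in progress.
; CompletedObjective switches the text to a completion message, plays a reverse animation after a short delay and clears the flag.
; The construction script sizes the box from BoxSize.
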(event OnComponentEndOverlap(ObjectiveBox)
  (params (OverlappedComponent :type Primitive%20Component%20Object%20Reference) (OtherActor :type Actor%20Object%20Reference) (OtherComp :type Primitive%20Component%20Object%20Reference) (OtherBodyIndex :type Integer))
  (bind _w_objectivewidgetref (Variables|Default|GetW_ObjectiveWidgetRef))
  (bind _w_objectivewidgetref_2 (Variables|Default|GetW_ObjectiveWidgetRef))
  (if (== OtherActor (Game|GetPlayerCharacter 0))
    (Utilities|FlowControl|DoOnce false
      (:Completed
        (Variables|/Game/Blueprints/W_Objetivo.W_Objetivo_C|SetObjectiveTextTitle _w_objectivewidgetref (Variables|Default|GetObjectiveTitleText))
        (Variables|/Game/Blueprints/W_Objetivo.W_Objetivo_C|SetObjectiveTextContent _w_objectivewidgetref (Variables|Default|GetObjectiveTitleContent))
        (Appearance|SetColorandOpacity (Variables|/Game/Blueprints/W_Objetivo.W_Objetivo_C|GetObjectiveContent _w_objectivewidgetref) (Utilities|Struct|MakeSlateColor (Utilities|Struct|MakeLinearColor 1.0 1.0 1.0 1.0) "UseColor_Specified") :!class /Script/UMG.TextBlock)
        (UserInterface|Viewport|AddtoViewport (stale EventBeginPlay _returnvalue) 0)
        (UserInterface|Animation|PlayAnimation _w_objectivewidgetref_2 (Variables|/Game/Blueprints/W_Objetivo.W_Objetivo_C|GetObjectiveFade _w_objectivewidgetref_2) 0.0 1 "Forward" 1.0 false)
        (Variables|Default|SetObjectiveInProgress? true)))))

(event Custom|CompletedObjective
  (bind _w_objectivewidgetref (Variables|Default|GetW_ObjectiveWidgetRef))
  (Variables|/Game/Blueprints/W_Objetivo.W_Objetivo_C|SetObjectiveTextContent _w_objectivewidgetref "Objetivo concluído")
  (Utilities|FlowControl|Delay 1.0)
  (UserInterface|Animation|PlayAnimation _w_objectivewidgetref 0 0.0 1 "Reverse" 1.0 false)
  (Variables|Default|SetObjectiveInProgress? false))

(event EventBeginPlay
  (bind _returnvalue (UserInterface|CreateWidget "/Game/Blueprints/W_Objetivo.W_Objetivo_C" 0 (Variables|Default|GetObjectiveTitleText) (Variables|Default|GetObjectiveTitleContent)))
  (Variables|Default|SetW_ObjectiveWidgetRef _returnvalue))

(event Collision|EventActorBeginOverlap
  (params (OtherActor :type Actor%20Object%20Reference)))

(event EventTick
  (params (DeltaSeconds :type Float%20%28single-precision%29)))

(fn ConstructionScript
  (Components|Box|SetBoxExtent (Variables|Default|GetObjective%20Box) (Variables|Default|GetBox%20Size) true))