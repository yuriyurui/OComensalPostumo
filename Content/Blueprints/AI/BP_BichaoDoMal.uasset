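; Enemy creature AI that stays dormant until the BP_StartTimer countdown ends, then roams between random "path1" actors.
; AI Perception makes it speed up and chase the player, but while BP_Armario (wardrobe) reports the player hidden, it forgets all targets and resumes patrol.
; Losing the player restores the slower speed and patrol.
; Sphere overlap with the player pauses the game and shows the W_MenuMorte death menu.
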(event OnTargetPerceptionUpdated(AIPerception)
  (params (Actor :type Actor%20Object%20Reference) (Stimulus :type AI%20Stimulus%20Structure))
  ;[0.15 0.15 0.15 0.5] Make the creature follow player
  (if (Variables|Default|GetFinishedTimer?)
    (if (Variables|/Game/Blueprints/BP_Armario.BP_Armario_C|GetisPlayerHidden (Variables|Default|GetArmario))
      (Class|AIPerceptionComponent|ForgetAll (Variables|Default|GetAIPerception))
      (CallFunction|Patrol)
      (else
        (Development|PrintString "Achei")
        (bind _asbp_player (Utilities|Casting|CastToBP_Player Actor))
        (Variables|/Script/Engine.CharacterMovementComponent|SetMaxWalkSpeed (Variables|Character|GetCharacterMovement) 3e+02)
        (AI|AIMoveTo self "0, 0, 0" _asbp_player 5.0 false)))))

(event OnTargetPerceptionForgotten(AIPerception)
  (params (Actor :type Actor%20Object%20Reference))
  ;[0.15 0.15 0.15 0.5] Make the creature go back to patrol function after forget player
  (Utilities|Casting|CastToBP_Player Actor)
  (Variables|/Script/Engine.CharacterMovementComponent|SetMaxWalkSpeed (Variables|Character|GetCharacterMovement) 2.5e+02)
  (if (Variables|Default|GetFinishedTimer?)
    (CallFunction|Patrol)))

(event OnComponentBeginOverlap(Sphere)
  (params (OverlappedComponent :type Primitive%20Component%20Object%20Reference) (OtherActor :type Actor%20Object%20Reference) (OtherComp :type Primitive%20Component%20Object%20Reference) (OtherBodyIndex :type Integer) (bFromSweep :type Boolean) (SweepResult :type Hit%20Result%20Structure%20%28by%20ref%29))
  (if (== OtherActor (Game|GetPlayerCharacter 0))
    (Utilities|FlowControl|DoOnce false
      (:Completed
        (Game|SetGamePaused true)
        (bind _returnvalue (UserInterface|CreateWidget "/Game/Blueprints/W_MenuMorte.W_MenuMorte_C"))
        (UserInterface|Viewport|AddtoViewport _returnvalue 0)
        (Variables|/Script/Engine.PlayerController|SetbShowMouseCursor (Game|GetPlayerController 0) true)))))

(event Custom|TimerFinished
  (Variables|Default|SetFinishedTimer? true))

(event Custom|Patrol
  ;[0.15 0.15 0.15 0.5] Make the creature patrol / move between points
  (bind _outactors (Actor|GetAllActorswithTag "path1"))
  (AI|AIMoveTo self "0, 0, 0" (.OutItem (Utilities|Array|Random _outactors)) 5.0 false
    (:OnSuccess
      (Utilities|FlowControl|Delay 1.0)
      (CallFunction|Patrol))))

(event EventBeginPlay
  (bind _returnvalue (Actor|GetActorOfClass "/Game/Blueprints/BP_Armario.BP_Armario_C"))
  (bind _asbp_armario (Utilities|Casting|CastToBP_Armario _returnvalue))
  (Variables|Default|SetArmario _asbp_armario)
  (Utilities|FlowControl|Delay 0.2)
  (bind _returnvalue_2 (Actor|GetActorOfClass "/Game/Blueprints/BP_StartTimer.BP_StartTimer_C"))
  (EventDispatchers|BindEventtoOnCountdownFinished (Variables|/Game/Blueprints/BP_StartTimer.BP_StartTimer_C|GetW_TimerRef _returnvalue_2) (delegate Custom|TimerFinished)))

(event EventTick
  (params (DeltaSeconds :type Float%20%28single-precision%29))
  (if (Variables|Default|GetFinishedTimer?)
    (Utilities|FlowControl|DoOnce false
      (:Completed
        (CallFunction|Patrol)))))

(fn ConstructionScript)